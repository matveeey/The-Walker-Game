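; Collectable actor that signals proximity with a point light and a floating text tip.
; Overlap begin and end toggle the text and switch the light between active and default intensity, with the end reset skipped once picked.
; Tick turns the text toward the player camera while overlapped and hides it once IsPicked is true.
; IsPicked is never set here, and the DstLightIntensity change sits behind contradictory IsPicked checks.
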(event EventBeginPlay)

(event Collision|EventActorBeginOverlap
  (params (OtherActor :type Actor%20Object%20Reference))
  (CallFunction|SetLightIntensity (Variables|Default|GetPointLight) (Variables|Default|GetActiveLightIntensity))
  (Rendering|ToggleVisibility (Variables|Default|GetFloatingText) false))

(event EventTick
  (params (DeltaSeconds :type Float%20%28single-precision%29))
  (if (Variables|Default|GetbIsPicked)
    (Rendering|SetVisibility (Variables|Default|GetFloatingText) (Math|Conversions|ToBoolean(Integer) 0) false))
  ;[1 1 1] Collision check
  (if (!= (Utilities|Array|IsEmpty (Collision|GetOverlappingActors 0 :!class /Script/Engine.Actor)) true)
    ;[1 1 1] Picked check (we don't need tip if collectable is already taken)
    (if (!= (Variables|Default|GetbIsPicked) true)
      (Transformation|SetWorldRotation (Variables|Default|GetFloatingText) (Math|Rotator|FindLookatRotation (Transformation|GetActorLocation) (Transformation|GetActorLocation (Game|GetPlayerCameraManager 0))) false false)
      (if (Variables|Default|GetbIsPicked)
        (CallFunction|SetLightIntensity (Variables|Default|GetPointLight) (Variables|Default|GetDstLightIntensity))))))

(event Collision|EventActorEndOverlap
  (params (OtherActor :type Actor%20Object%20Reference))
  (if (!= (Variables|Default|GetbIsPicked) true)
    (CallFunction|SetLightIntensity (Variables|Default|GetPointLight) (Variables|Default|GetDefaultLightIntensity))
    (Rendering|ToggleVisibility (Variables|Default|GetFloatingText) false)))

(fn ConstructionScript)

(fn SetLightIntensity
  (params (LightActor :type Point%20Light%20Component%20Object%20Reference) (Intensity :type Float%20%28double-precision%29))
  (Rendering|Components|Light|SetIntensity LightActor Intensity))